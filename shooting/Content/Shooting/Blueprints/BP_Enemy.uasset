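; BP_Enemy is a shooter enemy that moves in a straight line and damages BP_Player on contact.
; At BeginPlay it picks a fixed direction, 30% toward the player and otherwise forward, and Tick moves it by Speed without sweeping.
; Overlapping the player calls TakeDamage and destroys the enemy.
; If the returned value is zero or below, it also destroys the player, pauses the game and shows WBP_GameOver with UI-only input.
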(event EventBeginPlay
  ;[1 1 1] 태어날때
  ; : 방향을 30% 확률로 플레이어 방향, 나머지는 앞 방향으로
  (if (< (Math|Random|RandomIntegerinRange 0 9) 3)
    (Variables|Default|SetDirection (Math|Vector|Normalize (- (Transformation|GetActorLocation (Game|Player|GetPlayerPawn 0)) (Transformation|GetActorLocation))))
    (else
      (Variables|Default|SetDirection (Transformation|GetActorForwardVector)))))

(event Collision|EventActorBeginOverlap
  (params (OtherActor :type Actor%20Object%20Reference))
  (bind _returnvalue (Game|GetPlayerController 0))
  ;[1 1 1] 플레이어와 부딪힌 순간 플레이어의 체력을 1 소모하고 싶다.
  (bind _asbp_player (Utilities|Casting|CastToBP_Player OtherActor))
  (bind _newhp (Default|TakeDamage _asbp_player))
  (if (<= _newhp 0)
    (Actor|DestroyActor _asbp_player)
    (Actor|DestroyActor)
    ;[1 1 1] 주인공이 파괴되었으니 게임오버 처리하고 싶다
    (Game|SetGamePaused true)
    (bind _returnvalue_2 (UserInterface|CreateWidget "/Game/Shooting/UI/WBP_GameOver.WBP_GameOver_C"))
    (UserInterface|Viewport|AddtoViewport _returnvalue_2 0)
    (Variables|/Script/Engine.PlayerController|SetbShowMouseCursor _returnvalue false)
    (Input|SetInputModeUIOnly _returnvalue 0 "DoNotLock" false)
    (else
      (Actor|DestroyActor))))

(event EventTick
  (params (DeltaSeconds :type Float%20%28single-precision%29))
  ;[1 1 1] 살아가면서 P = P0 + vt
  ; : 그 방향으로 이동하게 하고 싶다.
  (Transformation|SetActorLocation (+ (Transformation|GetActorLocation) (* (Variables|Default|GetSpeed) (Variables|Default|GetDirection) (Utilities|Time|GetWorldDeltaSeconds))) false false))

(event Collision|EventActorEndOverlap
  (params (OtherActor :type Actor%20Object%20Reference)))

(event EventEndPlay
  (params (EndPlayReason :type EEndPlayReason%20Enum :default "Destroyed"))
  ;[1 1 1] 죽는 순간
)

(event EventDestroyed
  ;[1 1 1] 죽는 순간
)

(fn ConstructionScript)