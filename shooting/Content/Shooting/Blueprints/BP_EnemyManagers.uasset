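; Enemy spawner for the shooting game that keeps spawning BP_Enemy actors at its Arrow component's transform.
; BeginPlay starts a timer on the MakeEnemy event with a random delay of a few seconds.
; Each MakeEnemy call spawns one enemy and sets the timer again with a new random delay, so spawn intervals vary.
; An older accumulated-time spawn check remains in the graph but is disconnected and never runs.
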(event Custom|MakeEnemy
  ;[1 1 1] 이벤트 형식으로 제작 - 시간 전부 랜덤
  (Game|SpawnActorfromClass "/Game/Shooting/Blueprints/BP_Enemy.BP_Enemy_C" (Transformation|GetWorldTransform (Variables|Default|GetArrow)) "Undefined" "MultiplyWithRoot" 0 0)
  (Utilities|Time|SetTimerbyEvent (delegate Custom|MakeEnemy) (Math|Random|RandomFloatinRange 1.0 3.0) true))

(event EventBeginPlay
  ;[1 1 1] 이벤트 형식으로 제작 - 시간 전부 랜덤
  (Utilities|Time|SetTimerbyEvent (delegate Custom|MakeEnemy) (Math|Random|RandomFloatinRange 1.0 3.0) true))

(event Collision|EventActorBeginOverlap
  (params (OtherActor :type Actor%20Object%20Reference)))

(event EventTick
  (params (DeltaSeconds :type Float%20%28single-precision%29)))

(fn ConstructionScript)